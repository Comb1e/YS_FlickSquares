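; BP_FlickPlate is an actor that links the flick board to the player character at startup.
; On BeginPlay, after a short delay, it caches the first ball, flick board and third-person character found in the level.
; It then makes the character the flick board's owner.
; The ball reference is stored but unused here, and the overlap event is an empty placeholder.
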(event `self.ReceiveBeginPlay`
  (`KismetSystemLibrary.Delay` 0.2)
  (bind _outactors (`GameplayStatics.GetAllActorsOfClass` "/Game/Blueprints/BP_Ball.BP_Ball_C"))
  (set `self.Ball` (`|GetArrayItem` _outactors))
  (bind _outactors_2 (`GameplayStatics.GetAllActorsOfClass` "/Game/Blueprints/BP_FP_Children/BP_FlickBoard.BP_FlickBoard_C"))
  (bind _output_get (set `self.FlickBoard` (`|GetArrayItem` _outactors_2)))
  (bind _outactors_3 (`GameplayStatics.GetAllActorsOfClass` "/Game/Blueprints/BP_ThirdPersonCharacter.BP_ThirdPersonCharacter_C"))
  (bind _output_get_2 (set `self.MainCharacter` (`|GetArrayItem` _outactors_3)))
  (`self.SetOwner` _output_get _output_get_2))

(fn `UserConstructionScript`)