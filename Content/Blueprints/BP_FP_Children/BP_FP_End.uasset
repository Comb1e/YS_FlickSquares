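; BP_FP_End is a child Blueprint that acts as a fail zone, counting down remaining tries when the ball hits it.
; On a collision hit from the ball, it sets the main character's ball-attach flag and picks the ball's material from the current element type (thunder, water, fire, ice).
; It then decrements RemainTimes, and at zero prints a failure message and quits the game after a short delay.
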(event `self.CollisionComponent.OnComponentHit`
  (params (HitComponent :type "PrimitiveComponent Object Reference") (OtherActor :type "Actor Object Reference") (OtherComp :type "PrimitiveComponent Object Reference") (NormalImpulse :type "Vector Structure") (Hit :type "HitResult Structure (by ref)"))
  (if (== OtherActor (`self.Ball`))
    (set `/Game/Blueprints/BP_ThirdPersonCharacter.IfBallAttach` true (`self.MainCharacter`))
    (`PrimitiveComponent.SetMaterial` (`/Game/Blueprints/BP_Ball.Ball` (`self.Ball`)) 0 (select `int` (`/Game/Blueprints/BP_ThirdPersonCharacter.CurrentElementType` (`self.MainCharacter`)) :`0` "/Game/Materials/M_Ball_Inst/M_Ball_Thunder.M_Ball_Thunder" :`1` "/Game/Materials/M_Ball_Inst/M_Ball_Water.M_Ball_Water" :`2` "/Game/Materials/M_Ball_Inst/M_Ball_Fire.M_Ball_Fire" :`3` "/Game/Materials/M_Ball_Inst/M_Ball_Ice.M_Ball_Ice" :!type "MaterialInterface Object Reference"))
    (bind _output_get (set `self.RemainTimes` (- (`self.RemainTimes`) 1)))
    (if (== _output_get 0)
      (`KismetSystemLibrary.PrintString` "你失败了")
      (`KismetSystemLibrary.Delay` 1.0)
      (`KismetSystemLibrary.QuitGame` null "Quit"))))

(fn `UserConstructionScript`
  (`parent.UserConstructionScript`))