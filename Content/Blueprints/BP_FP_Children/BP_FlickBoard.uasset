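; BP_FlickBoard is a board owned by the third-person character that deflects the ball and passes on the character's element.
; Each tick it caches its owner as MainCharacter.
; On hit, it yaws the ball's projectile velocity in proportion to the board cube's Y velocity.
; If elements differ, the ball takes the character's element and material; a Water-Ice pairing also attaches it to the character at its current Y offset.
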(event `self.ReceiveTick`
  (params (DeltaSeconds :type "Float (single-precision)"))
  (`parent.ReceiveTick` DeltaSeconds)
  (bind _asbp_third_person_character (cast `/Game/Blueprints/BP_ThirdPersonCharacter` (`self.GetOwner`)))
  (set `self.MainCharacter` _asbp_third_person_character))

(event `self.CollisionComponent.OnComponentHit`
  (params (HitComponent :type "PrimitiveComponent Object Reference") (OtherActor :type "Actor Object Reference") (OtherComp :type "PrimitiveComponent Object Reference") (NormalImpulse :type "Vector Structure") (Hit :type "HitResult Structure (by ref)"))
  (bind _maincharacter (`self.MainCharacter`))
  (bind _currentelementtype (`/Game/Blueprints/BP_ThirdPersonCharacter.CurrentElementType` _maincharacter))
  (bind _projectilemovement (`/Game/Blueprints/BP_Ball.ProjectileMovement` (`self.Ball`)))
  (bind (_returnvalue_x _returnvalue_y) (`KismetMathLibrary.BreakVector` (`SceneComponent.K2_GetComponentLocation` (`Character.Mesh` (`self.MainCharacter`)))))
  (bind (_returnvalue_x_2 _returnvalue_y_2) (`KismetMathLibrary.BreakVector` (`SceneComponent.K2_GetComponentLocation` (`/Game/Blueprints/BP_Ball.Ball` (`self.Ball`)))))
  (bind _currentelementtype_2 (`/Game/Blueprints/BP_Ball.CurrentElementType` (`/Game/Blueprints/BP_ThirdPersonCharacter.Ball` _maincharacter)))
  (bind _returnvalue (`PrimitiveComponent.GetPhysicsLinearVelocity` (`self.Cube`) "None"))
  (set `MovementComponent.Velocity` (`KismetMathLibrary.GreaterGreater_VectorRotator` (`MovementComponent.Velocity` _projectilemovement) (`KismetMathLibrary.MakeRotator` 0.0 0.0 (* (/ (.y _returnvalue) 250.0) -15.0))) _projectilemovement)
  (if (not (== _currentelementtype _currentelementtype_2))
    (if (or (== _currentelementtype_2 1) (== _currentelementtype_2 3))
      (if (or (== (`/Game/Blueprints/BP_ThirdPersonCharacter.CurrentElementType` (`self.MainCharacter`)) 1) (== (`/Game/Blueprints/BP_ThirdPersonCharacter.CurrentElementType` (`self.MainCharacter`)) 3))
        (set `/Game/Blueprints/BP_ThirdPersonCharacter.BallOffset` (- _returnvalue_y_2 _returnvalue_y) (`self.MainCharacter`))
        (set `/Game/Blueprints/BP_ThirdPersonCharacter.IfBallAttach` true (`self.MainCharacter`))))
    (set `/Game/Blueprints/BP_Ball.CurrentElementType` _currentelementtype (`/Game/Blueprints/BP_ThirdPersonCharacter.Ball` (`self.MainCharacter`)))
    (`PrimitiveComponent.SetMaterial` (`/Game/Blueprints/BP_Ball.Ball` (`self.Ball`)) 0 (select `int` _currentelementtype :`0` "/Game/Materials/M_Ball_Inst/M_Ball_Thunder.M_Ball_Thunder" :`1` "/Game/Materials/M_Ball_Inst/M_Ball_Water.M_Ball_Water" :`2` "/Game/Materials/M_Ball_Inst/M_Ball_Fire.M_Ball_Fire" :`3` "/Game/Materials/M_Ball_Inst/M_Ball_Ice.M_Ball_Ice" :!type "MaterialInterface Object Reference"))))

(fn `UserConstructionScript`
  (`parent.UserConstructionScript`))