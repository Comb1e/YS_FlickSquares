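; BP_Ball is a projectile ball, owned by the third-person character, that flags BP_FP_Block actors to break based on element types.
; Each Tick while detached and in one of two element types, it box-traces forward and checks the first hit, plus the second when equidistant.
; CheckSCBreak sets IfSCBreak on very close, unfrozen blocks whose element differs from the ball's but belongs to the same pair.
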(event `self.ReceiveTick`
  (params (DeltaSeconds :type "Float (single-precision)"))
  (bind _returnvalue (`SceneComponent.K2_GetComponentLocation` (`self.Ball`)))
  (`|ExecutionSequence`
    (:`then_1`
      (bind _asbp_third_person_character (cast `/Game/Blueprints/BP_ThirdPersonCharacter` (`self.GetOwner`)))
      (if (`/Game/Blueprints/BP_ThirdPersonCharacter.IfBallAttach` _asbp_third_person_character)
        _
        (elif (or (== (`self.CurrentElementType`) 0) (== 3 (`self.CurrentElementType`)))
          (bind _outhits (`KismetSystemLibrary.BoxTraceMulti` _returnvalue (+ _returnvalue (* (`SceneComponent.GetForwardVector` (`self.Ball`)) 1000.0)) (20.0 20.0 1.0) (struct) "TraceTypeQuery1"))
          (bind _output_get (set `self.OutHits` _outhits))
          (if (`KismetArrayLibrary.Array_IsValidIndex` _output_get)
            (bind (_bblockinghit _binitialoverlap _time _distance _location _impactpoint _normal _impactnormal _physmat _hitactor) (`GameplayStatics.BreakHitResult` (`|GetArrayItem` _output_get)))
            (bind _asbp_fp_block (cast `/Game/Blueprints/BP_FP_Children/BP_FP_Block` _hitactor))
            (`self.CheckSCBreak` _asbp_fp_block _distance)
            (if (`KismetArrayLibrary.Array_IsValidIndex` _output_get 1)
              (bind (_bblockinghit_2 _binitialoverlap_2 _time_2 _distance_2 _location_2 _impactpoint_2 _normal_2 _impactnormal_2 _physmat_2 _hitactor_2) (`GameplayStatics.BreakHitResult` (`|GetArrayItem` _output_get 1)))
              (bind _asbp_fp_block_2 (cast `/Game/Blueprints/BP_FP_Children/BP_FP_Block` _hitactor_2))
              (if (== _distance_2 _distance)
                (`self.CheckSCBreak` _asbp_fp_block_2 _distance_2)))))))))

(fn `CheckSCBreak`
  (params (FP_Block :type "/Game/Blueprints/BP_FP_Children/BP_FP_Block Object Reference") (dist :type "Float (double-precision)"))
  (bind _currentelementtype (`/Game/Blueprints/BP_FP_Children/BP_FP_Block.CurrentElementType` FP_Block))
  (if (and (not (`/Game/Blueprints/BP_FP_Children/BP_FP_Block.IfFrozen` FP_Block)) (not (== (`self.CurrentElementType`) _currentelementtype)) (or (== 0 _currentelementtype) (== 3 _currentelementtype)) (< dist 35.0))
    (set `/Game/Blueprints/BP_FP_Children/BP_FP_Block.IfSCBreak` true FP_Block)))

(fn `UserConstructionScript`)